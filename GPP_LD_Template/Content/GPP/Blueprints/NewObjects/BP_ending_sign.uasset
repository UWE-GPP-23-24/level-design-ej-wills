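; An ending sign trigger that shows a tutorial message and plays a one-time camera cinematic when the player walks into its box.
; Overlap creates a WB_Tutorial widget displaying the Info text, which is collapsed when the overlap ends.
; On the first completed run, it disables character movement, blends the view through three Core targets on timed delays, then restores walking and the player view.
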(event OnComponentBeginOverlap(Box)
  (params (OverlappedComponent :type Primitive%20Component%20Object%20Reference) (OtherActor :type Actor%20Object%20Reference) (OtherComp :type Primitive%20Component%20Object%20Reference) (OtherBodyIndex :type Integer) (bFromSweep :type Boolean) (SweepResult :type Hit%20Result%20Structure%20%28by%20ref%29))
  (bind _returnvalue (Game|GetPlayerController 0))
  (bind _returnvalue_2 (Game|GetPlayerController 0))
  (bind _asbp_player_character (Utilities|Casting|CastToBP_PlayerCharacter OtherActor))
  (bind _returnvalue_3 (UserInterface|CreateWidget "/Game/GPP/Blueprints/NewObjects/WB_Tutorial.WB_Tutorial_C" _returnvalue_2))
  (bind _output_get (Variables|Default|SettutorialRef _returnvalue_3))
  (Variables|/Game/GPP/Blueprints/NewObjects/WB_Tutorial.WB_Tutorial_C|SetText (Variables|Default|GettutorialRef) (Variables|Default|GetInfo))
  (UserInterface|Viewport|AddtoViewport _output_get 0)
  (Widget|SetVisibility _output_get "Visible")
  (Utilities|FlowControl|Delay 0.2)
  (if (not (Variables|Default|Getcinematic_used))
    (Class|CameraComponent|GetCameraView (Variables|/Game/GPP/Blueprints/Essential/BP_PlayerCharacter.BP_PlayerCharacter_C|GetFollowCamera _asbp_player_character) 0.0)
    (Game|Player|SetViewTargetwithBlend _returnvalue_2 (Variables|Default|GetCore%20one) 2.0 "VTBlend_EaseInOut" 1.0 false)
    (Pawn|Components|CharacterMovement|SetMovementMode (Variables|/Script/Engine.Character|GetCharacterMovement _asbp_player_character) "MOVE_None" 0)
    (Utilities|FlowControl|Delay 3.0)
    (Game|Player|SetViewTargetwithBlend _returnvalue_2 (Variables|Default|GetCore%20two) 2.0 "VTBlend_EaseIn" 0.5 false)
    (Utilities|FlowControl|Delay 3.0)
    (Game|Player|SetViewTargetwithBlend _returnvalue (Variables|Default|GetCore%20three) 2.0 "VTBlend_EaseIn" 0.5 false)
    (Utilities|FlowControl|Delay 3.0)
    (Pawn|Components|CharacterMovement|SetMovementMode (Variables|/Script/Engine.Character|GetCharacterMovement _asbp_player_character) "MOVE_Walking" 0)
    (Game|Player|SetViewTargetwithBlend _returnvalue _asbp_player_character 2.0 "VTBlend_EaseIn" 0.5 false)
    (Variables|Default|Setcinematic_used true)))

(event OnComponentEndOverlap(Box)
  (params (OverlappedComponent :type Primitive%20Component%20Object%20Reference) (OtherActor :type Actor%20Object%20Reference) (OtherComp :type Primitive%20Component%20Object%20Reference) (OtherBodyIndex :type Integer))
  (Widget|SetVisibility (Variables|Default|GettutorialRef) "Collapsed"))

(event EventBeginPlay)

(event EventTick
  (params (DeltaSeconds :type Float%20%28single-precision%29)))

(fn ConstructionScript)