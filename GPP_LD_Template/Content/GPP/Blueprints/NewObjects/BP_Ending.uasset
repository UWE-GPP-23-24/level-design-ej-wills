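; BP_Ending is an actor that tracks collected cores and reacts when the player reaches it with the required number.
; Collectcore increments CollectedInt, and its trailing branch does nothing.
; When BP_PlayerCharacter overlaps Box and CollectedInt exactly equals CoresNeeded, it sets IsCollected, unhides the actor and disables Box collision.
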(event OnComponentBeginOverlap(Box)
  (params (OverlappedComponent :type Primitive%20Component%20Object%20Reference) (OtherActor :type Actor%20Object%20Reference) (OtherComp :type Primitive%20Component%20Object%20Reference) (OtherBodyIndex :type Integer) (bFromSweep :type Boolean) (SweepResult :type Hit%20Result%20Structure%20%28by%20ref%29))
  (Utilities|Casting|CastToBP_PlayerCharacter OtherActor)
  (if (== (Variables|Default|GetCores_Needed) (Variables|Default|Getcollected%20int))
    (Variables|Default|SetIs_collected true)
    (Rendering|SetActorHiddenInGame false)
    (Collision|SetCollisionEnabled (Variables|Default|GetBox) "NoCollision")))

(event Custom|Collect%20core
  (Math|Integer|IncrementInt (Variables|Default|Getcollected%20int)
    (:%20%20
      (if true
        _))))

(event EventBeginPlay)

(event Collision|EventActorBeginOverlap
  (params (OtherActor :type Actor%20Object%20Reference)))

(event EventTick
  (params (DeltaSeconds :type Float%20%28single-precision%29)))

(fn ConstructionScript)