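; A floor actor that temporarily vanishes when a linked explosive barrel's fuse runs out.
; Each Tick it polls the referenced Barrel for a triggered state and a nearly expired fuse timer.
; After a short delay it hides itself and disables collision, then restores both after a longer delay.
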(event EventBeginPlay)

(event Collision|EventActorBeginOverlap
  (params (OtherActor :type Actor%20Object%20Reference)))

(event EventTick
  (params (DeltaSeconds :type Float%20%28single-precision%29))
  (bind _barrel (Variables|Default|GetBarrel))
  (Utilities|IsValid (Variables|Default|GetBarrel)
    (:Is%20Valid
      (if (and (Variables|/Game/GPP/Blueprints/Obstacles/BP_ExplodingBarrels.BP_ExplodingBarrels_C|GetIsTriggered _barrel) (<= (Variables|/Game/GPP/Blueprints/Obstacles/BP_ExplodingBarrels.BP_ExplodingBarrels_C|GetFuseTimer _barrel) 0.1))
        (Utilities|FlowControl|Delay 0.15)
        (Rendering|SetActorHiddenInGame true)
        (Collision|SetActorEnableCollision false)
        (Utilities|FlowControl|Delay 1e+01)
        (Rendering|SetActorHiddenInGame false)
        (Collision|SetActorEnableCollision true)))))

(fn ConstructionScript)