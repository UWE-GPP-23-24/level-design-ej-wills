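; BP_Help_sign_noCinematic is a help sign trigger that shows tutorial text while the player is nearby, with no cinematic in its logic.
; When BP_PlayerCharacter enters its Box, it creates a WB_Tutorial widget, fills it with the Info text and displays it.
; Any end overlap collapses the stored widget without an actor check or removal, so each player entry adds a new widget.
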(event OnComponentBeginOverlap(Box)
  (params (OverlappedComponent :type Primitive%20Component%20Object%20Reference) (OtherActor :type Actor%20Object%20Reference) (OtherComp :type Primitive%20Component%20Object%20Reference) (OtherBodyIndex :type Integer) (bFromSweep :type Boolean) (SweepResult :type Hit%20Result%20Structure%20%28by%20ref%29))
  (Utilities|Casting|CastToBP_PlayerCharacter OtherActor)
  (bind _returnvalue (UserInterface|CreateWidget "/Game/GPP/Blueprints/NewObjects/WB_Tutorial.WB_Tutorial_C" (Game|GetPlayerController 0)))
  (bind _output_get (Variables|Default|SettutorialRef _returnvalue))
  (Variables|/Game/GPP/Blueprints/NewObjects/WB_Tutorial.WB_Tutorial_C|SetText (Variables|Default|GettutorialRef) (Variables|Default|GetInfo))
  (UserInterface|Viewport|AddtoViewport _output_get 0)
  (Widget|SetVisibility _output_get "Visible"))

(event OnComponentEndOverlap(Box)
  (params (OverlappedComponent :type Primitive%20Component%20Object%20Reference) (OtherActor :type Actor%20Object%20Reference) (OtherComp :type Primitive%20Component%20Object%20Reference) (OtherBodyIndex :type Integer))
  (Widget|SetVisibility (Variables|Default|GettutorialRef) "Collapsed"))

(event EventBeginPlay)

(event EventTick
  (params (DeltaSeconds :type Float%20%28single-precision%29)))

(fn ConstructionScript)